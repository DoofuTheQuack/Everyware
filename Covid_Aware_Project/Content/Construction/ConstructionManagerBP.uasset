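; Construction manager that queues timed building placements and swaps each proxy for the finished building.
; QueueBuild spawns a proxy with the display mesh, binds its completion event, stores it alongside its config in parallel arrays, and sets its build time in hours.
; On completion, FinishBuild looks up the config by proxy index, removes both entries, spawns the building at the stored transform and destroys the proxy.
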(event `BindBuildComplete`
  (params (Proxy :type "/Game/Construction/ConstructionProxyBP Object Reference"))
  (add `/Game/Construction/ConstructionProxyBP.BuildCompleted` Proxy (`|CreateDelegate` :!event `BuildCompleted`)))

(event `BuildCompleted`
  (params (Proxy :type "/Game/Construction/ConstructionProxyBP Object Reference"))
  (`self.FinishBuild` Proxy))

(fn `FinishBuild`
  (params (Proxy :type "/Game/Construction/ConstructionProxyBP Object Reference"))
  (locals (Index :type Integer) (Config :type "/Game/Construction/Construction_Struct Structure"))
  (bind (_buildingclass _proxyclass _transform) (break `/Game/Construction/Construction_Struct` (`local.Config`)))
  (bind _output_get (set `local.Index` (`KismetArrayLibrary.Array_Find` (`self.Proxies`) Proxy)))
  (set `local.Config` (`|GetArrayItem` (`self.ConStructures`) _output_get))
  (`KismetArrayLibrary.Array_Remove` (`self.ConStructures`) (`local.Index`))
  (`KismetArrayLibrary.Array_Remove` (`self.Proxies`) (`local.Index`))
  (`|SpawnActorFromClass` _buildingclass _transform "Undefined" "OverrideRootScale" null null null)
  (`self.K2_DestroyActor` Proxy))

(fn `QueueBuild`
  (params (ConStruct :type "/Game/Construction/Construction_Struct Structure"))
  (bind (_buildingclass _proxyclass _transform _displaymesh _hours) (break `/Game/Construction/Construction_Struct` ConStruct))
  (bind _returnvalue (`|SpawnActorFromClass` _proxyclass _transform "Undefined" "OverrideRootScale" null _displaymesh null))
  (`self.BindBuildComplete` _returnvalue)
  (`KismetArrayLibrary.Array_Add` (`self.Proxies`) _returnvalue)
  (`KismetArrayLibrary.Array_Add` (`self.ConStructures`) ConStruct)
  (`/Game/Construction/ConstructionProxyBP.SetBuildTime` _returnvalue _hours))

(fn `UserConstructionScript`)