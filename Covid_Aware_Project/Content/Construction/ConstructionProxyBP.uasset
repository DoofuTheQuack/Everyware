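; Construction placeholder actor for an RTS that shows a building's mesh in a ghost material until its build completes.
; It binds to the RTS game state's game-speed updates, and each Tick calls Build, which only fetches a clockwork value from that state.
; When BuildTimeTotal, which no visible logic increments, exceeds the hours-based BuildTime, it fires BuildCompleted and destroys itself after a short delay.
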(event `self.ReceiveBeginPlay`
  (bind _asrtsgamestate (cast `/Game/GameState/RTSGamestate` (`GameplayStatics.GetGameState`)))
  (bind _output_get (set `self.GameStateRef` _asrtsgamestate))
  (add `/Game/GameState/RTSGamestate.UpdateGameSpeed` _output_get (`|CreateDelegate` :!event `AdjustTime`)))

(event `AdjustTime`
  (params (TimeUnits :type "Float (double-precision)"))
  (set `self.TimeUnits` TimeUnits))

(event `self.ReceiveTick`
  (params (DeltaSeconds :type "Float (single-precision)"))
  (set `self.Delta` DeltaSeconds)
  (if (not (`self.IsBuildCompleted`))
    (`self.Build`)
    (if (> (`self.BuildTimeTotal`) (`self.BuildTime`))
      (set `self.IsBuildCompleted` true)
      (`self.BuildCompleted` self)
      (`KismetSystemLibrary.Delay` 0.2)
      (`self.K2_DestroyActor`))))

(fn `Build`
  (set `self.Clock` (`/Game/GameState/RTSGamestate.SetCLockwork` (`self.GameStateRef`) (`self.Delta`))))

(fn `SetBuildTime`
  (params (Hours :type "Float (double-precision)"))
  (set `self.BuildTime` (* Hours 60.0))
  (return))

(fn `UserConstructionScript`
  (bind _staticmesh (`self.StaticMesh`))
  (`StaticMeshComponent.SetStaticMesh` _staticmesh (`self.DisplayMesh`))
  (`PrimitiveComponent.SetMaterial` _staticmesh 0 "/Game/Buildings/PlacementTXT/GhostMatInst.GhostMatInst"))