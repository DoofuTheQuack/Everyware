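; Placement preview actor for build mode that shows a ghost mesh of the chosen building at the grid-snapped cursor position.
; ConstructObject spawns the building class to read its mesh and construction proxy, then enables build mode and a gated Tick.
; Tick checks overlaps, then line-traces corners and center for slope, box-tracing to set height, and swaps to an error material when invalid.
; GetConstructionStruct packages class, proxy, transform and mesh.
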(event `Kill`
  ;[1 1 1] Kill
  (set `self.BuildingClass` null)
  (set `self.ConstructionProxy` null)
  (`self.CloseTick`)
  (set `self.DisplayMesh` null)
  (set `self.IsActive?` false)
  (set `/Game/CameraController/CameraPawnController.BuildMode` false (`self.CameraControllerRef`))
  (`StaticMeshComponent.SetStaticMesh` (`self.GhostMesh`) (`self.DisplayMesh`))
  (`self.K2_SetActorRotation` (struct)))

(event `Spawn`
  (params (DisplayMesh :type "StaticMesh Object Reference") (BuildingClass :type "/Game/Buildings/BuildingMasterBP Class Reference") (ConstructionProxy :type "/Game/Construction/ConstructionProxyBP Class Reference"))
  ;[1 1 1] On Spawn
  (if (not (`self.IsActive?`))
    (set `self.BuildingClass` BuildingClass)
    (set `self.ConstructionProxy` ConstructionProxy)
    (set `self.IsActive?` true)
    (bind _output_get (set `self.DisplayMesh` DisplayMesh))
    (`StaticMeshComponent.SetStaticMesh` (`self.GhostMesh`) _output_get)
    (`self.OpenTick`)
    (`self.SetMaterial` (not (`self.IsOverlapping?`)))
    (set `self.Extent` (`.BoxExtent` (`KismetSystemLibrary.GetComponentBounds` (`self.GhostMesh`))))))

(event `/Game/Interfaces/I_HUD.Construct Object`
  (params (Buildin :type "/Game/Buildings/BuildingMasterBP Class Reference"))
  ;[1 1 1] Construct
  (bind _returnvalue (`|SpawnActorFromClass` Buildin (`KismetMathLibrary.MakeTransform` (0.0 0.0 0.0)) "Undefined" "OverrideRootScale" null (`self.CameraControllerRef`) (`self.DisplayMesh`) 5.0 0.0 null))
  (`|ExecutionSequence`
    (:`then_0`
      (`self.Kill`)
      (bind _asbuilding_master_bp (castclass `/Game/Buildings/BuildingMasterBP` Buildin))
      (set `/Game/CameraController/CameraPawnController.BuildMode` true (`self.CameraControllerRef`))
      (`self.Spawn` (`/Game/Buildings/BuildingMasterBP.DisplayMesh` _returnvalue) _asbuilding_master_bp (`/Game/Buildings/BuildingMasterBP.ConstructionProxy` _returnvalue)))
    (:`then_1`
      (`self.K2_DestroyActor`))))

(event `self.ReceiveTick`
  (params (DeltaSeconds :type "Float (single-precision)"))
  (bind _snap (`self.SetGridSnapVector`))
  ;[1 1 1] OnTick
  (`/Engine/EditorBlueprintResources/StandardMacros.Gate` true :!label _label
    (:`Exit`
      (`self.K2_SetActorLocation` self _snap false false)
      (`KismetSystemLibrary.PrintString` (`KismetStringLibrary.Conv_VectorToString` _snap))
      (if (`self.CheckOverlap`)
        (`self.SetMaterial` true)
        (else
          (bind _bad (`self.CheckSlope`))
          (`self.SetMaterial` _bad))))))

(event `OpenTick`
  ;[1 1 1] OnTick
  (goto _label :!via `Open`))

(event `CloseTick`
  ;[1 1 1] OnTick
  (goto _label :!via `Close`))

(event `SetMaterial`
  (params (Error :type Boolean))
  (bind _ghostmesh (`self.GhostMesh`))
  ;[1 1 1] SetInstMaterial
  (if (not (== Error (`self.IsOverlapping?`)))
    (bind _output_get (set `self.IsOverlapping?` Error))
    (if _output_get
      (`PrimitiveComponent.SetMaterial` _ghostmesh 0 "/Game/Buildings/PlacementTXT/GhostMathErrorInst.GhostMathErrorInst")
      (else
        (`PrimitiveComponent.SetMaterial` _ghostmesh 0 "/Game/Buildings/PlacementTXT/GhostMatInst.GhostMatInst")))))

(fn `CheckOverlap`
  (returns (Overlap :type Boolean))
  (return (> (`KismetArrayLibrary.Array_Length` (`self.GetOverlappingActors` self "/Script/Engine.Actor")) 0)))

(fn `CheckSlope`
  (returns (Bad :type Boolean))
  (locals (Diffs :type "Array of Float (double-precision)") (MaxDiffs :type "Float (double-precision)"))
  (bind (_actorlocation _forwardvector _rightvector) (`self.GetVectors`))
  (bind _actorlocation_2 (`self.GetVectors`))
  (bind _actorlocation_3 (`self.GetVectors`))
  (bind (_actorlocation_4 _forwardvector_2 _rightvector_2) (`self.GetVectors`))
  (bind (_actorlocation_5 _forwardvector_3 _rightvector_3) (`self.GetVectors`))
  (bind (_actorlocation_6 _forwardvector_4 _rightvector_4) (`self.GetVectors`))
  (bind _diffs (`local.Diffs`))
  (bind _maxdiffs (`local.MaxDiffs`))
  (bind (_extent_x _extent_y) (`KismetMathLibrary.BreakVector` (`self.Extent`)))
  (bind (_indexofminvalue _minvalue) (`KismetMathLibrary.MinOfFloatArray` _diffs))
  (bind (_indexofmaxvalue _maxvalue) (`KismetMathLibrary.MaxOfFloatArray` _diffs))
  (`|ExecutionSequence`
    (:`then_0`
      (`|ExecutionSequence`
        (:`then_0`
          (bind _diff (`self.SlopeTrace` (+ _actorlocation_4 (* (+ _forwardvector_2 _rightvector_2) (`self.Extent`)))))
          (`KismetArrayLibrary.Array_Add` (`local.Diffs`) _diff))
        (:`then_1`
          (bind _diff_2 (`self.SlopeTrace` (+ _actorlocation_5 (* (+ (* _forwardvector_3 -1.0) _rightvector_3) (`self.Extent`)))))
          (`KismetArrayLibrary.Array_Add` (`local.Diffs`) _diff_2))
        (:`then_2`
          (bind _diff_3 (`self.SlopeTrace` (+ _actorlocation_6 (* (+ _forwardvector_4 (* _rightvector_4 -1.0)) (`self.Extent`)))))
          (`KismetArrayLibrary.Array_Add` (`local.Diffs`) _diff_3))
        (:`then_3`
          (bind _diff_4 (`self.SlopeTrace` (+ _actorlocation (* (+ (* _forwardvector -1.0) (* _rightvector -1.0)) (`self.Extent`)))))
          (`KismetArrayLibrary.Array_Add` (`local.Diffs`) _diff_4))
        (:`then_4`
          (bind _diff_5 (`self.SlopeTrace` (`self.GetVectors`)))
          (`KismetArrayLibrary.Array_Add` (`local.Diffs`) _diff_5))))
    (:`then_1`
      (if (and (> _indexofminvalue -1) (> _indexofmaxvalue -1))
        (bind (_outhit _returnvalue) (`KismetSystemLibrary.BoxTraceSingle` (+ _actorlocation_3 (0.0 0.0 1000.0)) (- _actorlocation_3 (0.0 0.0 1000.0)) (`KismetMathLibrary.MakeVector` _extent_x _extent_y 1.0) (struct) "TraceTypeQuery3"))
        (if _returnvalue
          (`self.K2_SetActorLocation` (`KismetMathLibrary.MakeVector` (.x _actorlocation_2) (.y _actorlocation_2) (.z (`.ImpactPoint` (`GameplayStatics.BreakHitResult` _outhit))))))))
    (:`then_2`
      (return (or (> (`KismetMathLibrary.Abs` _minvalue) _maxdiffs) (> (`KismetMathLibrary.Abs` _maxvalue) _maxdiffs))))))

(fn `GetConstructionStruct`
  (returns (ConstructionStructure :type "/Game/Construction/Construction_Struct Structure"))
  (return (make `/Game/Construction/Construction_Struct` (`self.BuildingClass`) (`self.ConstructionProxy`) (`KismetMathLibrary.MakeTransform` (`self.K2_GetActorLocation`) (`self.K2_GetActorRotation`)) (`self.DisplayMesh`))))

(fn `GetIsOverlapping`
  (returns (Overlapping :type Boolean))
  (return (`self.IsOverlapping?`)))

(fn `GetVectors`
  (returns (ActorLocation :type "Vector Structure") (ForwardVector :type "Vector Structure") (RightVector :type "Vector Structure"))
  (bind _returnvalue (`self.K2_GetActorRotation`))
  (return (`self.K2_GetActorLocation`) (`KismetMathLibrary.GetForwardVector` _returnvalue) (`KismetMathLibrary.GetRightVector` _returnvalue)))

(fn `SetCalander`
  (params (Date :type "Array of Integer (by ref)"))
  (returns (Success :type Boolean))
  (return false))

(fn `SetClock`
  (params (Time :type "Array of Integer (by ref)"))
  (returns (Success :type Boolean))
  (return false))

(fn `SetCursorPosition`
  (params (Position :type "Vector Structure"))
  (returns (CursorPos :type "Vector Structure"))
  (bind _output_get (set `self.CursorWorldPosition` Position))
  (return _output_get))

(fn `SetGridSnapVector`
  (returns (Snap :type "Vector Structure"))
  (bind (_cursorworldposition_x _cursorworldposition_y _cursorworldposition_z) (`KismetMathLibrary.BreakVector` (`self.CursorWorldPosition`)))
  (bind _gridsize (`self.GridSize`))
  (return (`KismetMathLibrary.MakeVector` (`/Game/GameState/FunctionLibrary.GridSnap` _cursorworldposition_x _gridsize) (`/Game/GameState/FunctionLibrary.GridSnap` _cursorworldposition_y _gridsize) (`/Game/GameState/FunctionLibrary.GridSnap` _cursorworldposition_z _gridsize))))

(fn `SlopeTrace`
  (params (Location :type "Vector Structure"))
  (returns (Diff :type "Float (double-precision)"))
  (bind (_returnvalue_x _returnvalue_y _returnvalue_z) (`KismetMathLibrary.BreakVector` (`self.K2_GetActorLocation`)))
  (bind _outhit (`KismetSystemLibrary.LineTraceSingle` (+ Location (0.0 0.0 1000.0)) (- Location (0.0 0.0 1000.0)) "TraceTypeQuery3"))
  (return (- _returnvalue_z (.z (`.ImpactPoint` (`GameplayStatics.BreakHitResult` _outhit))))))

(fn `UserConstructionScript`)